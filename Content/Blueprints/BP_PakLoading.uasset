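; Runtime pak loader that mounts pak files in packaged builds and brings their assets into the world.
; LoadPackFile validates and mounts the pak, then registers its content path, logs its files and loads its AssetRegistry.
; Spawn events resolve filenames to package names to play sounds, spawn meshes or Blueprint actors, and apply textures to BP_Pic.
; BP_TestPawn's mouse hit supplies spawn locations and the actor receiving materials.
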(event Custom|LoadPackFile
  (params (PakFilename :type String) (Log%20File%20Path :type String) (Mount%20Point :type String) (Pak%20Directory :type String) (Root%20Path :type String) (MountEasy? :type Boolean))
  (Variables|Default|SetPakFilePath PakFilename)
  (Variables|Default|SetNew%20Log%20Path Log%20File%20Path)
  (Variables|Default|SetMountPoint Mount%20Point)
  (Variables|Default|SetPak%20Directory Pak%20Directory)
  (Variables|Default|SetRoot%20Path Root%20Path)
  (Variables|Default|SetMount%20Easy? MountEasy?)
  (if (Class|PakLoaderLibrary|IsPackagedBuild)
    (Class|PakLoaderLibrary|EnableRuntimeLog true (Variables|Default|GetNew%20Log%20Path))
    (Class|PakLoaderLibrary|RuntimeLog (Utilities|String|Append (Variables|Default|GetPakFilePath) " : " (Variables|Default|GetNew%20Log%20Path) " : " (Variables|Default|GetMountPoint) " : " (Variables|Default|GetPak%20Directory) " : " (Variables|Default|GetRoot%20Path)))
    (bind _returnvalue (Class|PakLoaderLibrary|IsValidPakFile (Variables|Default|GetPakFilePath)))
    (if _returnvalue
      (Class|PakLoaderLibrary|RuntimeLog (Utilities|String|Append (Variables|Default|GetPakFilePath) "     Pak is OK"))
      (if (Variables|Default|GetMount%20Easy?)
        (bind _returnvalue_2 (Class|PakLoaderLibrary|MountPakFileEasy (Variables|Default|GetPakFilePath)))
        (Class|PakLoaderLibrary|RuntimeLog (Utilities|String|Append "Easy Mount Pak File Successfull : " (Utilities|String|ToString(Boolean) _returnvalue_2)))
        (CallFunction|RegisterMountPoint _returnvalue_2)
        (else
          (bind _returnvalue_3 (Class|PakLoaderLibrary|MountPakFile (Variables|Default|GetPakFilePath) (Variables|Default|GetMountPoint)))
          (Class|PakLoaderLibrary|RuntimeLog (Utilities|String|Append "Mount Pak File Successfull : " (Utilities|String|ToString(Boolean) _returnvalue_3)))
          (CallFunction|RegisterMountPoint _returnvalue_3)))
      (else
        (Class|PakLoaderLibrary|RuntimeLog (Utilities|String|Append (Variables|Default|GetPakFilePath) " PakFile invalid"))))
    (else
      (Development|PrintString "Not a packaged build"))))

(event Custom|Spawn%20BP
  (params (Filename :type String))
  (bind (_packagename _returnvalue) (Class|PakLoaderLibrary|TryConvertFilenametoLongPackageName Filename))
  ;[0.15 0.15 0.15 0.5] Spawn BP form pak file
  (Class|PakLoaderLibrary|RuntimeLog (Utilities|String|Append _packagename "  =  " (Utilities|String|ToString(Boolean) _returnvalue)))
  (bind _asactor (Utilities|Casting|CastToActorClass (Class|PakLoaderLibrary|GetPakFileClass _packagename))
    (:then
      (Class|PakLoaderLibrary|RuntimeLog (Utilities|String|Append "CAst Successfull     " (Utilities|GetClassDisplayName _asactor)))
      (bind _returnvalue_2 (Game|SpawnActorfromClass _asactor (Math|Transform|MakeTransform (.Location (Collision|BreakHitResult (Variables|Default|GetHit%20Result))) "0, 0, 0" "1.000000,1.000000,1.000000") "Undefined" "SelectDefaultAtRuntime" 0 0))
      (Class|PakLoaderLibrary|RuntimeLog (Utilities|GetDisplayName _returnvalue_2)))
    (:CastFailed
      (Class|PakLoaderLibrary|RuntimeLog "Cast Fail"))))

(event Custom|Spawn%20Texture
  (params (Filename :type String))
  (bind (_packagename _returnvalue) (Class|PakLoaderLibrary|TryConvertFilenametoLongPackageName Filename))
  ;[0.15 0.15 0.15 0.5] Spawn Texture From Pak File
  (bind _returnvalue_2 (Actor|GetActorOfClass "/Game/Blueprints/BP_Pic.BP_Pic_C"))
  (Class|PakLoaderLibrary|RuntimeLog (Utilities|String|Append _packagename "  =  " (Utilities|String|ToString(Boolean) _returnvalue)))
  (Default|SetNewTexture _returnvalue_2 (Class|PakLoaderLibrary|GetPakFileTexture2D _packagename)))

(event Custom|Spawn%20Static%20Mesh
  (params (Filename :type String))
  (bind (_packagename _returnvalue) (Class|PakLoaderLibrary|TryConvertFilenametoLongPackageName Filename))
  ;[0.15 0.15 0.15 0.5] Spawn Static Mesh From pak file
  (bind _returnvalue_2 (Game|SpawnActorfromClass "/Script/Engine.StaticMeshActor" (Math|Transform|MakeTransform (.Location (Collision|BreakHitResult (Variables|Default|GetHit%20Result))) "0, 0, 0" "1.000000,1.000000,1.000000") "Undefined" "MultiplyWithRoot" 0 0))
  (Class|PakLoaderLibrary|RuntimeLog (Utilities|String|Append _packagename "  =  " (Utilities|String|ToString(Boolean) _returnvalue)))
  (Transformation|SetMobility (Variables|/Script/Engine.StaticMeshActor|GetStaticMeshComponent _returnvalue_2) "Movable")
  (bind _returnvalue_3 (Components|StaticMesh|SetStaticMesh (Variables|/Script/Engine.StaticMeshActor|GetStaticMeshComponent _returnvalue_2) (Class|PakLoaderLibrary|GetPakFileStaticMesh _packagename)))
  (Class|PakLoaderLibrary|RuntimeLog (Utilities|String|Append "Static Mesh Spawned  :    " (Utilities|String|ToString(Boolean) _returnvalue_3))))

(event Custom|Spawn%20Music
  (params (Filename :type String))
  (bind (_packagename _returnvalue) (Class|PakLoaderLibrary|TryConvertFilenametoLongPackageName Filename))
  ;[0.15 0.15 0.15 0.5] Spawn Music From PAK File
  (Class|PakLoaderLibrary|RuntimeLog (Utilities|String|Append _packagename "  =  " (Utilities|String|ToString(Boolean) _returnvalue)))
  (Audio|PlaySound2D (Class|PakLoaderLibrary|GetPakFileSound _packagename) 1.0 1.0 0.0 0 0))

(event Custom|Spawn%20Skeletal%20Mesh
  (params (Filename :type String))
  (bind (_packagename _returnvalue) (Class|PakLoaderLibrary|TryConvertFilenametoLongPackageName Filename))
  ;[0.15 0.15 0.15 0.5] Spawn Skeletol Mesh From Pak File
  (bind _returnvalue_2 (Game|SpawnActorfromClass "/Script/Engine.SkeletalMeshActor" (Math|Transform|MakeTransform (.Location (Collision|BreakHitResult (Variables|Default|GetHit%20Result))) "0, 0, 0" "1.000000,1.000000,1.000000") "Undefined" "MultiplyWithRoot" 0 0))
  (Class|PakLoaderLibrary|RuntimeLog (Utilities|String|Append _packagename "  =  " (Utilities|String|ToString(Boolean) _returnvalue)))
  (Components|SkeletalMesh|SetSkeletalMeshAsset (Variables|/Script/Engine.SkeletalMeshActor|GetSkeletalMeshComponent _returnvalue_2) (Class|PakLoaderLibrary|GetPakFileSkeletalMesh _packagename)))

(event Custom|Spawn%20Material
  (params (Filename :type String) (Material%20Index :type Integer))
  (bind (_packagename _returnvalue) (Class|PakLoaderLibrary|TryConvertFilenametoLongPackageName Filename))
  (bind _hit_result (Variables|Default|GetHit%20Result))
  (bind _hitactor (Collision|BreakHitResult _hit_result))
  (bind _returnvalue_2 (Class|PakLoaderLibrary|GetPakFileMaterial _packagename))
  ;[0.15 0.15 0.15 0.5] Spawn Material Form Pak File
  (Variables|Default|SetMaterial%20Index Material%20Index)
  (Class|PakLoaderLibrary|RuntimeLog (Utilities|String|Append _packagename "  =  " (Utilities|String|ToString(Boolean) _returnvalue)))
  (Utilities|IsValid _returnvalue_2
    (:Is%20Valid
      (bind _output_get (Variables|Default|SetMaterial _returnvalue_2))
      (Class|PakLoaderLibrary|RuntimeLog (Utilities|String|Append "Material :  " (Utilities|GetDisplayName _output_get)))
      (CallFunction|SetMaterialtoReleventSelectedObject _hitactor (Variables|Default|GetMaterial) (Variables|Default|GetMaterial%20Index)))
    (:Is%20Not%20Valid
      (bind _output_get_2 (Variables|Default|SetMaterial%20Instance (Class|PakLoaderLibrary|GetPakFileMaterialInstanceConstant _packagename)))
      (Class|PakLoaderLibrary|RuntimeLog (Utilities|String|Append "Material Instance : " (Utilities|GetDisplayName _output_get_2)))
      (CallFunction|SetMaterialtoReleventSelectedObject _hitactor (Variables|Default|GetMaterial%20Instance) (Variables|Default|GetMaterial%20Index)))))

(event Custom|Register%20Mount%20Point
  (params (Condition :type Boolean))
  (if Condition
    (Class|PakLoaderLibrary|RegisterMountPoint (Utilities|String|Append "/" (Variables|Default|GetRoot%20Path) "/") (Utilities|String|Append (Variables|Default|GetMountPoint) "Content/"))
    (Utilities|FlowControl|Sequence
      (:then_0
        (CallFunction|ListMountedPakFileNmaes))
      (:then_1
        (CallFunction|ListFilesinPakDirectory))
      (:then_2
        (Class|PakLoaderLibrary|RuntimeLog (Utilities|String|Append "Pak Directory Esist : " (Utilities|String|ToString(Boolean) (Class|PakLoaderLibrary|DoesPakDirectoryExist (Variables|Default|GetMountPoint))))))
      (:then_3
        (Class|PakLoaderLibrary|LoadPakAssetRegistryFile (Utilities|String|Append (Variables|Default|GetMountPoint) "/AssetRegistry.bin"))
        (Class|PakLoaderLibrary|RuntimeLog "Populated pak assets to Unreal's AssetRegistry")))
    (else
      (Class|PakLoaderLibrary|RuntimeLog "Failed to mount pak, stopping..."))))

(event Custom|OnMouse%20Point_Event
  (params (HitResult :type Hit%20Result%20Structure))
  (Variables|Default|SetHit%20Result HitResult))

(event EventBeginPlay
  (bind _asbp_test_pawn (Utilities|Casting|CastToBP_TestPawn (Game|Player|GetPlayerPawn 0)))
  (EventDispatchers|AssignOnMousePoint _asbp_test_pawn (delegate Custom|OnMouse%20Point_Event)))

(fn ConstructionScript)

(fn GetActorLocation
  (params (Tag :type Name))
  (bind _outactors (Actor|GetAllActorsOfClasswithTag "/Game/Blueprints/BP_SpawnPoint.BP_SpawnPoint_C" Tag))
  (return (Transformation|GetActorLocation (Utilities|Array|Get(acopy) _outactors))))

(fn ListMountedPakFileNmaes
  (for _array_element (Class|PakLoaderLibrary|GetMountedPakFilenames)
    (Class|PakLoaderLibrary|RuntimeLog (Utilities|String|Append "Pak File Name :) ->   " _array_element)))
  (Class|PakLoaderLibrary|RuntimeLog " 
"))

(fn ListFilesinPakDirectory
  (bind _returnvalue (Class|PakLoaderLibrary|GetFilesinPakDirectory (Variables|Default|GetPak%20Directory) true))
  (for _array_element _returnvalue
    (if (not (or (Utilities|Enum|Equal(Enum) (Class|BlueprintPathsLibrary|GetExtension _array_element false) "uexp") (Utilities|Enum|Equal(Enum) (Class|BlueprintPathsLibrary|GetExtension _array_element false) "ubulk"))) ; Filter uexp/ubulk files
      (if (.ReturnValue (Class|PakLoaderLibrary|TryConvertFilenametoLongPackageName _array_element))
        (Class|PakLoaderLibrary|RuntimeLog (Utilities|String|Append "FIle In the Pak Directory :)   ->    " (.PackageName (Class|PakLoaderLibrary|TryConvertFilenametoLongPackageName _array_element))))
        (else
          (Class|PakLoaderLibrary|RuntimeLog "Failed to list files in the pak directory"))))))

(fn SetMaterialtoReleventSelectedObject
  (params (Actor :type Actor%20Object%20Reference) (InMaterial :type Material%20Interface%20Object%20Reference) (ElementIndex :type Integer))
  (bind _returnvalue (Actor|GetComponentbyClass Actor "/Script/Engine.SkeletalMeshComponent"))
  (bind _returnvalue_2 (Actor|GetComponentbyClass Actor "/Script/Engine.StaticMeshComponent"))
  (bind _asstatic_mesh_actor (Utilities|Casting|CastToStaticMeshActor Actor)
    (:then
      (Rendering|Material|SetMaterial (Variables|/Script/Engine.StaticMeshActor|GetStaticMeshComponent _asstatic_mesh_actor) ElementIndex InMaterial))
    (:CastFailed
      (bind _asskeletal_mesh_actor (Utilities|Casting|CastToSkeletalMeshActor Actor)
        (:then
          (Rendering|Material|SetMaterial (Variables|/Script/Engine.SkeletalMeshActor|GetSkeletalMeshComponent _asskeletal_mesh_actor) ElementIndex InMaterial))
        (:CastFailed
          (Utilities|IsValid _returnvalue_2
            (:Is%20Valid
              (Rendering|Material|SetMaterial _returnvalue_2 ElementIndex InMaterial))
            (:Is%20Not%20Valid
              (Utilities|IsValid _returnvalue
                (:Is%20Valid
                  (Rendering|Material|SetMaterial _returnvalue ElementIndex InMaterial))))))))))