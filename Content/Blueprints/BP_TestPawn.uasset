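; Test pawn that adds the WBP_Main widget to the viewport and shows the mouse cursor on BeginPlay.
; The 1 key and right mouse button both fire MouseLocation, which deprojects the cursor and line-traces into the world on the Visibility channel.
; On a hit, it calls OnMousePoint with the hit result and spawns a BP_Pointer at the impact point.
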(event Custom|Mouse%20Location
  (bind _returnvalue (Game|GetPlayerController 0))
  (bind (_worldlocation _worlddirection) (Game|Player|ConvertMouseLocationToWorldSpace _returnvalue))
  (bind (_outhit _returnvalue_2) (Collision|LineTraceByChannel _worldlocation (+ _worldlocation (* _worlddirection 5e+03)) "TraceTypeQuery1" false 0 "None"))
  (if _returnvalue_2
    (bind _output_get (Variables|Default|SetOut%20Hit _outhit))
    (Default|CallOnMousePoint _output_get)
    (Game|SpawnActorfromClass "/Game/Blueprints/BP_Pointer.BP_Pointer_C" (Math|Transform|MakeTransform (.ImpactPoint (Collision|BreakHitResult _output_get)) "0, 0, 0" "1.000000,1.000000,1.000000") "Undefined" "MultiplyWithRoot" 0 0)))

(event EventBeginPlay
  (bind _returnvalue (UserInterface|CreateWidget "/Game/Blueprints/WBP_Main.WBP_Main_C"))
  (UserInterface|Viewport|AddtoViewport _returnvalue 0)
  (Variables|/Script/Engine.PlayerController|SetbShowMouseCursor (Game|GetPlayerController 0) true))

(event Input|MouseEvents|RightMouseButton
  (params (Key :type Key%20Structure :default "None"))
  (:Pressed
    (CallFunction|MouseLocation)))

(event Input|KeyboardEvents|1
  (params (Key :type Key%20Structure :default "None"))
  (:Pressed
    (CallFunction|MouseLocation)))

(fn ConstructionScript)